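; BP_Spill is a floor spill that makes the first-person player slippery and can be mopped up.
; Box overlap lowers the tagged player's braking and acceleration, and leaving sets TurnOffSlip on the character instead of restoring values here.
; Each Mop call adds to the player's MoppedAmount and slightly shrinks the Cube in X and Y, destroying the spill once both reach a minimum.
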(event `Mop`
  (params (player :type "/Game/FirstPerson/Blueprints/BP_FirstPersonCharacter Object Reference"))
  (bind _cube (`self.Cube`))
  (bind (_returnvalue_x _returnvalue_y _returnvalue_z) (`KismetMathLibrary.BreakVector` (`SceneComponent.K2_GetComponentScale` _cube)))
  (if (and (<= _returnvalue_x 1.5) (<= _returnvalue_y 1.5))
    (`self.K2_DestroyActor`)
    (else
      (bind _output_get (set `/Game/FirstPerson/Blueprints/BP_FirstPersonCharacter.moppedAmount` (+ (stale _output_get) 0.05) player))
      (`KismetSystemLibrary.PrintString` (`KismetStringLibrary.Conv_DoubleToString` _output_get))
      (`SceneComponent.SetWorldScale3D` _cube (`KismetMathLibrary.MakeVector` (- _returnvalue_x 0.005) (- _returnvalue_y 0.005) _returnvalue_z)))))

(event `self.Box.OnComponentBeginOverlap`
  (params (OverlappedComponent :type "PrimitiveComponent Object Reference") (OtherActor :type "Actor Object Reference") (OtherComp :type "PrimitiveComponent Object Reference") (OtherBodyIndex :type Integer) (bFromSweep :type Boolean) (SweepResult :type "HitResult Structure (by ref)"))
  (`KismetSystemLibrary.PrintString` (`KismetSystemLibrary.GetDisplayName` OtherActor))
  (if (`self.ActorHasTag` OtherActor "Player")
    (bind _asbp_first_person_character (cast `/Game/FirstPerson/Blueprints/BP_FirstPersonCharacter` OtherActor))
    (bind _charactermovement (`Character.CharacterMovement` _asbp_first_person_character))
    (set `CharacterMovementComponent.BrakingFrictionFactor` 0.0 _charactermovement)
    (set `CharacterMovementComponent.BrakingDecelerationWalking` 100.0 _charactermovement)
    (set `CharacterMovementComponent.MaxAcceleration` 500.0 _charactermovement)))

(event `self.Box.OnComponentEndOverlap`
  (params (OverlappedComponent :type "PrimitiveComponent Object Reference") (OtherActor :type "Actor Object Reference") (OtherComp :type "PrimitiveComponent Object Reference") (OtherBodyIndex :type Integer))
  (if (`self.ActorHasTag` OtherActor "Player")
    (bind _asbp_first_person_character (cast `/Game/FirstPerson/Blueprints/BP_FirstPersonCharacter` OtherActor))
    (set `/Game/FirstPerson/Blueprints/BP_FirstPersonCharacter.turnOffSlip` true _asbp_first_person_character)))

(fn `UserConstructionScript`)