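; Rubbish bin actor that collects objects tagged as spillable and tracks how full it is as a percentage.
; Box overlap destroys spillable objects and calls AddRubbsh, which raises the fill (stored in WaterAmount) while below 100 and updates the text.
; Box1 overlap shows or hides that text for the player and sets or clears the character's NearbyBin reference.
; While the player is nearby, Tick rotates the text to face them.
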(event `AddRubbsh`
  (params (rubbishAmount :type "Float (double-precision)"))
  (if (< (`self.waterAmount`) 100.0)
    (bind _output_get (set `self.waterAmount` (+ (stale _output_get) rubbishAmount)))
    (`TextRenderComponent.K2_SetText` (`self.TextRender`) (`KismetSystemLibrary.MakeLiteralText` (`|FormatText` "Rubbsh \nAmount \n{0}%" _output_get)))))

(event `self.Box1.OnComponentBeginOverlap`
  (params (OverlappedComponent :type "PrimitiveComponent Object Reference") (OtherActor :type "Actor Object Reference") (OtherComp :type "PrimitiveComponent Object Reference") (OtherBodyIndex :type Integer) (bFromSweep :type Boolean) (SweepResult :type "HitResult Structure (by ref)"))
  (if (`self.ActorHasTag` OtherActor "Player")
    (`SceneComponent.SetVisibility` (`self.TextRender`) true false)
    (bind _asbp_first_person_character (cast `/Game/FirstPerson/Blueprints/BP_FirstPersonCharacter` OtherActor))
    (set `/Game/FirstPerson/Blueprints/BP_FirstPersonCharacter.nearbyBin` self _asbp_first_person_character)
    (set `self.playerNearby` true)
    (set `self.nearbyPlayer` OtherActor)))

(event `self.ReceiveTick`
  (params (DeltaSeconds :type "Float (single-precision)"))
  (if (`self.playerNearby`)
    (`SceneComponent.K2_SetWorldRotation` (`self.TextRender`) (`KismetMathLibrary.FindLookAtRotation` (`self.K2_GetActorLocation`) (`self.K2_GetActorLocation` (`self.nearbyPlayer`))) false false)))

(event `self.Box1.OnComponentEndOverlap`
  (params (OverlappedComponent :type "PrimitiveComponent Object Reference") (OtherActor :type "Actor Object Reference") (OtherComp :type "PrimitiveComponent Object Reference") (OtherBodyIndex :type Integer))
  (if (`self.ActorHasTag` OtherActor "Player")
    (`SceneComponent.SetVisibility` (`self.TextRender`) false false)
    (bind _asbp_first_person_character (cast `/Game/FirstPerson/Blueprints/BP_FirstPersonCharacter` OtherActor))
    (set `/Game/FirstPerson/Blueprints/BP_FirstPersonCharacter.nearbyBin` null _asbp_first_person_character)
    (set `self.playerNearby` false)
    (set `self.nearbyPlayer` null)))

(event `self.Box.OnComponentBeginOverlap`
  (params (OverlappedComponent :type "PrimitiveComponent Object Reference") (OtherActor :type "Actor Object Reference") (OtherComp :type "PrimitiveComponent Object Reference") (OtherBodyIndex :type Integer) (bFromSweep :type Boolean) (SweepResult :type "HitResult Structure (by ref)"))
  (if (`self.ActorHasTag` OtherActor "spillableobject")
    (`self.K2_DestroyActor` OtherActor)
    (`self.AddRubbsh` 5.0)))

(fn `UserConstructionScript`)