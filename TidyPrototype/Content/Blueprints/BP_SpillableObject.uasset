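; BP_SpillableObject is a physics object that leaves a spill when it lands on the floor.
; Its Cube starts simulating physics on BeginPlay.
; When the Cube hits an actor tagged "floor" while the object is not equipped, it stops simulating, switches to query-only collision and spawns a BP_Spill using the Cube's X and Y location.
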(event `self.ReceiveBeginPlay`
  (`PrimitiveComponent.SetSimulatePhysics` (`self.Cube`) true))

(event `self.Cube.OnComponentHit`
  (params (HitComponent :type "PrimitiveComponent Object Reference") (OtherActor :type "Actor Object Reference") (OtherComp :type "PrimitiveComponent Object Reference") (NormalImpulse :type "Vector Structure") (Hit :type "HitResult Structure (by ref)"))
  (bind (_returnvalue_x _returnvalue_y) (`KismetMathLibrary.BreakVector` (`SceneComponent.K2_GetComponentLocation` (`self.Cube`))))
  (if (`self.equipped`)
    _
    (elif (`self.ActorHasTag` OtherActor "floor")
      (`PrimitiveComponent.SetSimulatePhysics` (`self.Cube`) false)
      (`PrimitiveComponent.SetCollisionEnabled` (`self.Cube`) "QueryOnly")
      (`|SpawnActorFromClass` "/Game/Blueprints/BP_Spill.BP_Spill_C" (`KismetMathLibrary.MakeTransform` (`KismetMathLibrary.MakeVector` _returnvalue_x _returnvalue_y)) "Undefined" "MultiplyWithRoot" null null))))

(fn `UserConstructionScript`)